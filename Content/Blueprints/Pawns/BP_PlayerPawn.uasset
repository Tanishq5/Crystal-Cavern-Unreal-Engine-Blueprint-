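; Player pawn that moves by applying torque to its physics mesh and restarts the level when damaged.
; The forward/backward and right/left input axes add Speed-scaled torque around Y and X as an acceleration change, independent of mass.
; BeginPlay fades the camera in from black.
; The first damage event, gated by DoOnce, fades the camera out, holds it, then reopens the current level after a matching delay.
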(event `self.ReceiveBeginPlay`
  (`PlayerCameraManager.StartCameraFade` :`self` (`GameplayStatics.GetPlayerCameraManager` 0) :`FromAlpha` 1.0 :`Duration` 3.0))

(event `InputAxis|Move Forwar/Backward`
  (params (AxisValue :type "Float (single-precision)"))
  (`PrimitiveComponent.AddTorqueInRadians` (`self.mesh`) (`KismetMathLibrary.MakeVector` 0.0 (* AxisValue (`self.Speed`))) "None" true))

(event `InputAxis|Move Right/Left`
  (params (AxisValue :type "Float (single-precision)"))
  (`PrimitiveComponent.AddTorqueInRadians` (`self.mesh`) (`KismetMathLibrary.MakeVector` (* AxisValue (`self.Speed`))) "None" true))

(event `self.ReceiveAnyDamage`
  (params (Damage :type "Float (single-precision)") (DamageType :type "DamageType Object Reference") (InstigatedBy :type "Controller Object Reference") (DamageCauser :type "Actor Object Reference"))
  (`/Engine/EditorBlueprintResources/StandardMacros.DoOnce` false
    (:`Completed`
      (`PlayerCameraManager.StartCameraFade` :`self` (`GameplayStatics.GetPlayerCameraManager` 0) :`ToAlpha` 1.0 :`Duration` 1.0 :`bHoldWhenFinished` true)
      (`KismetSystemLibrary.Delay` 1.0)
      (bind _returnvalue (`GameplayStatics.GetCurrentLevelName` true))
      (`GameplayStatics.OpenLevel` (`KismetStringLibrary.Conv_StringToName` _returnvalue)))))

(fn `UserConstructionScript`)