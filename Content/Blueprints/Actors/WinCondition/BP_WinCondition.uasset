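; BP_WinCondition is a level exit actor that advances the game to the next level once all crystals are gone.
; When the player pawn overlaps it and no BP_Crystal actors remain, it completes the level.
; It finds the current level in a LevelNames array and opens the following entry by name, doing nothing further on the final level.
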(event `self.ReceiveActorBeginOverlap`
  (params (OtherActor :type "Actor Object Reference"))
  (if (== OtherActor (`GameplayStatics.GetPlayerPawn` 0))
    (bind _outactors (`GameplayStatics.GetAllActorsOfClass` "/Game/Blueprints/Actors/collectables/BP_Crystal.BP_Crystal_C"))
    (if (not (> (`KismetArrayLibrary.Array_Length` _outactors) 0))
      (`self.Complete Level`))))

(fn `Complete Level`
  (if (not (`self.Is Final Level`))
    (`self.Load Next Level`)))

(fn `Get Current Level Name`
  (returns (`Return Value` :type Integer))
  (bind _returnvalue (`GameplayStatics.GetCurrentLevelName` true))
  (return (`KismetArrayLibrary.Array_Find` (`self.Level Names`) (`KismetStringLibrary.Conv_StringToName` _returnvalue))))

(fn `Get Next Level Name`
  (returns (`Return Value` :type Name))
  (return (`|GetArrayItem` (`self.Level Names`) (+ (`self.Get Current Level Name`) 1))))

(fn `Is Final Level`
  (returns (`Return Value` :type Boolean))
  (return (== (`KismetArrayLibrary.Array_LastIndex` (`self.Level Names`)) (`self.Get Current Level Name`))))

(fn `Load Next Level`
  (`GameplayStatics.OpenLevel` (`self.Get Next Level Name`)))

(fn `UserConstructionScript`)